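; BP_Test_DestructibleObj is a test destructible object built on a Chaos Geometry Collection cube that speeds up an enemy when broken.
; On the Chaos break event it turns off physics simulation on the cube, waits briefly, then calls Die.
; Die destroys the actor and calls IncreaseSpeed on the BP_Enemy returned by GetActorOfClass.
; The overlap event is empty and the kinematic field calls are unconnected.
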(event `self.GC_Cube.OnComponentBeginOverlap`
  (params (OverlappedComponent :type "PrimitiveComponent Object Reference") (OtherActor :type "Actor Object Reference") (OtherComp :type "PrimitiveComponent Object Reference") (OtherBodyIndex :type Integer) (bFromSweep :type Boolean) (SweepResult :type "HitResult Structure (by ref)")))

(event `self.GC_Cube.OnChaosBreakEvent`
  (params (BreakEvent :type "ChaosBreakEvent Structure (by ref)"))
  (`PrimitiveComponent.SetSimulatePhysics` (`self.GC_Cube`) false)
  (`KismetSystemLibrary.Delay` 1.0)
  (`self.die`))

(fn `die`
  (`self.K2_DestroyActor`)
  (bind _returnvalue (`GameplayStatics.GetActorOfClass` "/Game/FieryInferno/BP_Enemy.BP_Enemy_C"))
  (`/Game/FieryInferno/BP_Enemy.Increase Speed` _returnvalue))

(fn `UserConstructionScript`)