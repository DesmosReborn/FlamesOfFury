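; CameraBP is an actor, named as a camera, that smoothly follows a FollowTarget.
; Each Tick calls Move, which uses VInterpTo to ease its location toward the target's position at InterpSpeed, without sweeping.
; A LockHeight flag keeps the actor's current Z so it follows only on the horizontal plane.
; Only location is updated; rotation is untouched.
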(event `self.ReceiveTick`
  (params (DeltaSeconds :type "Float (single-precision)"))
  (`self.Move`))

(fn `Move`
  (bind (_returnvalue_x _returnvalue_y _returnvalue_z) (`KismetMathLibrary.BreakVector` (`self.K2_GetActorLocation`)))
  (bind (_returnvalue_x_2 _returnvalue_y_2 _returnvalue_z_2) (`KismetMathLibrary.BreakVector` (`self.K2_GetActorLocation` (`self.followTarget`))))
  (`self.K2_SetActorLocation` (`KismetMathLibrary.VInterpTo` (`self.K2_GetActorLocation`) (`KismetMathLibrary.MakeVector` _returnvalue_x_2 _returnvalue_y_2 (select `bool` (`self.lockHeight`) :`false` _returnvalue_z_2 :`true` _returnvalue_z)) (`GameplayStatics.GetWorldDeltaSeconds`) (`self.interpSpeed`))))

(fn `UserConstructionScript`)